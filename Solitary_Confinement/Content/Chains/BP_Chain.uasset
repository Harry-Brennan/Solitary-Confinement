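; BP_Chain is a chain Blueprint that lays repeated copies of a mesh along a spline.
; Its construction script rebuilds an instanced static mesh component, deriving link spacing from half the mesh's X bounding size plus an offset.
; Spline length divided by that spacing sets the link count, and each instance takes its local position and rotation from the spline at that distance.
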(fn `UserConstructionScript`
  (locals (NumberOfInstances :type Integer :default 0))
  (bind _spline (`self.Spline`))
  (bind (_min _max) (break `Box` (`StaticMesh.GetBoundingBox` (`self.SM`))))
  (`InstancedStaticMeshComponent.ClearInstances` (`self.InstancedStaticMesh`))
  (`StaticMeshComponent.SetStaticMesh` (`self.InstancedStaticMesh`) (`self.SM`))
  (bind _output_get (set `self.Spacing` (+ (.x (/ (- _max _min) 2.0)) (`self.Offset`))))
  (bind _output_get_2 (set `local.NumberOfInstances` (`KismetMathLibrary.FFloor` (/ (`SplineComponent.GetSplineLength` (`self.Spline`)) _output_get))))
  (for _index (range (+ _output_get_2 1))
    (bind _returnvalue (* _index (`self.Spacing`)))
    (`InstancedStaticMeshComponent.AddInstance` (`self.InstancedStaticMesh`) (`KismetMathLibrary.MakeTransform` (`SplineComponent.GetLocationAtDistanceAlongSpline` _spline _returnvalue "Local") (`SplineComponent.GetRotationAtDistanceAlongSpline` _spline _returnvalue "Local")) false)))