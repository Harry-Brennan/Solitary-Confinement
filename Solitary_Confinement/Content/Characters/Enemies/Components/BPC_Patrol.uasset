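; BPC_Patrol is an enemy patrol component that tracks a target location along the spline of a PatrolActor.
; FindStartingPatrolLoc snaps the target to the closest spline location to the owner and rounds the nearest input key into the point index.
; UpdateSplineIndex increments that index, resetting to zero only after it exceeds the point count, and UpdatePatrolLoc converts it to a world-space PatrolLoc.
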(fn `Find_Starting_Patrol_Loc`
  (set `self.Patrol_Loc` (`SplineComponent.FindLocationClosestToWorldLocation` (`/Game/Characters/Enemies/BP_Enemy_Patrol.Spline` (`self.Patrol_Actor`)) (`Actor.K2_GetActorLocation` (`self.GetOwner`)) "World"))
  (set `self.Patrol_Spline_Index` (`KismetMathLibrary.Round` (`SplineComponent.FindInputKeyClosestToWorldLocation` (`/Game/Characters/Enemies/BP_Enemy_Patrol.Spline` (`self.Patrol_Actor`)) (`Actor.K2_GetActorLocation` (`self.GetOwner`))))))

(fn `Update_Patrol_Loc`
  (set `self.Patrol_Loc` (`SplineComponent.GetLocationAtSplinePoint` (`/Game/Characters/Enemies/BP_Enemy_Patrol.Spline` (`self.Patrol_Actor`)) (`self.Patrol_Spline_Index`) "World")))

(fn `Update_Spline_Index`
  (bind _patrol_spline_index (`self.Patrol_Spline_Index`))
  (if (> _patrol_spline_index (`SplineComponent.GetNumberOfSplinePoints` (`/Game/Characters/Enemies/BP_Enemy_Patrol.Spline` (`self.Patrol_Actor`))))
    (set `self.Patrol_Spline_Index` 0)
    (else
      (`/Engine/EditorBlueprintResources/StandardMacros.IncrementInt` _patrol_spline_index))))