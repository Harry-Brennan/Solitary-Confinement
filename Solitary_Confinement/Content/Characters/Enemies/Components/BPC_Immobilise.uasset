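; BPC_Immobilise is an enemy component that freezes its owning character in place and later releases it.
; Immobilise sets the Immobilised flag, disables the owner's character movement and applies an overlay material to its skeletal mesh as a visual cue.
; StopImmobilise clears the flag and overlay, and always returns movement to Walking rather than restoring the previous mode.
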(fn `Immobilise`
  (set `self.Immobilised` true)
  (`CharacterMovementComponent.DisableMovement` (`Actor.GetComponentByClass` (`self.GetOwner`) "/Script/Engine.CharacterMovementComponent"))
  (`MeshComponent.SetOverlayMaterial` (`Actor.GetComponentByClass` (`self.GetOwner`) "/Script/Engine.SkeletalMeshComponent") "/Game/Characters/Enemies/Materials/M_Enemy_Immobilise.M_Enemy_Immobilise"))

(fn `Stop_Immobilise`
  (set `self.Immobilised` false)
  (`CharacterMovementComponent.SetMovementMode` (`Actor.GetComponentByClass` (`self.GetOwner`) "/Script/Engine.CharacterMovementComponent") "MOVE_Walking" 0)
  (`MeshComponent.SetOverlayMaterial` (`Actor.GetComponentByClass` (`self.GetOwner`) "/Script/Engine.SkeletalMeshComponent") null))