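; Player actor component that rolls the view into sideways movement, adding a subtle strafe tilt to the camera.
; On BeginPlay it caches the owner's camera and the Character's controller.
; Each tick it converts velocity to local space, scales the lateral component into a target roll, then interpolates and clamps it to a few degrees.
; The roll is written through control rotation, skipping updates when pitch nears straight up or down.
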(event `self.ReceiveBeginPlay`
  (set `self.Camera` (`Actor.GetComponentByClass` (`self.GetOwner`) "/Script/Engine.CameraComponent"))
  (bind _ascharacter (cast `Character` (`self.GetOwner`)))
  (set `self.Controller` (`Pawn.GetController` _ascharacter)))

(event `self.ReceiveTick`
  (params (DeltaSeconds :type "Float (single-precision)"))
  (bind _returnvalue (`self.GetOwner`))
  (bind _controller (`self.Controller`))
  (bind (_returnvalue_roll _returnvalue_pitch) (`KismetMathLibrary.BreakRotator` (`Controller.GetControlRotation` (`self.Controller`))))
  (bind (_returnvalue_roll_2 _returnvalue_pitch_2 _returnvalue_yaw) (`KismetMathLibrary.BreakRotator` (`Controller.GetControlRotation` _controller)))
  (bind _returnvalue_roll_3 (`KismetMathLibrary.BreakRotator` (`SceneComponent.K2_GetComponentRotation` (`self.Camera`))))
  (bind (_returnvalue_x _returnvalue_y) (`KismetMathLibrary.BreakVector` (`KismetMathLibrary.LessLess_VectorRotator` (`Actor.GetVelocity` _returnvalue) (`Actor.K2_GetActorRotation` _returnvalue))))
  (if (not (or (and (>= _returnvalue_pitch 85.0) (<= _returnvalue_pitch 255.0)) (and (<= _returnvalue_pitch 275.0) (>= _returnvalue_pitch 255.0))))
    (`Controller.SetControlRotation` _controller (`KismetMathLibrary.MakeRotator` (`KismetMathLibrary.FClamp` (`KismetMathLibrary.FInterpTo` _returnvalue_roll_3 (* (/ _returnvalue_y 1000.0) 4.0) (`GameplayStatics.GetWorldDeltaSeconds`) 2.0) -4.0 4.0) _returnvalue_pitch_2 _returnvalue_yaw))))