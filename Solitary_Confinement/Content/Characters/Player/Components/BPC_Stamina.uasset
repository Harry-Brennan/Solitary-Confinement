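; Player stamina component that exposes functions to drain, regenerate and handle exhaustion of a stamina value.
; UseStamina and RegenStamina each move CurrentStamina one FInterpTo step per call, so outside code must call them repeatedly.
; NoStamina prints a warning and sets ShouldRegenStamina on BP_ThirdPersonCharacter, found by casting player 0's character; RegenStamina clears it near MaxStamina.
; Tick is empty, and a debug stamina print is disconnected.
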(event `self.ReceiveTick`
  (params (DeltaSeconds :type "Float (single-precision)")))

(fn `No_Stamina`
  (`KismetSystemLibrary.PrintString` "OUT OF STAMINA")
  (bind _asbp_third_person_character (cast `/Game/Characters/Player/BP_ThirdPersonCharacter` (`GameplayStatics.GetPlayerCharacter` 0)))
  (set `/Game/Characters/Player/BP_ThirdPersonCharacter.Should_Regen_Stamina` true _asbp_third_person_character))

(fn `Regen_Stamina`
  (set `self.Current_Stamina` (`KismetMathLibrary.FInterpTo` (`self.Current_Stamina`) (`self.Max_Stamina`) (`GameplayStatics.GetWorldDeltaSeconds`) 3.0))
  (if (>= (`self.Current_Stamina`) (- (`self.Max_Stamina`) 1.0))
    (set `self.Current_Stamina` (`self.Max_Stamina`))
    (bind _asbp_third_person_character (cast `/Game/Characters/Player/BP_ThirdPersonCharacter` (`GameplayStatics.GetPlayerCharacter` 0)))
    (set `/Game/Characters/Player/BP_ThirdPersonCharacter.Should_Regen_Stamina` false _asbp_third_person_character)))

(fn `Use_Stamina`
  (if (not (<= (`self.Current_Stamina`) 0.01))
    (set `self.Current_Stamina` (`KismetMathLibrary.FInterpTo` (`self.Current_Stamina`) (- (`self.Current_Stamina`) 10.0) (`GameplayStatics.GetWorldDeltaSeconds`) 5.0))))