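; Player component that picks the enemy the camera is aimed at and highlights it with an outline overlay material.
; Each tick it line-traces forward from the owner's camera, storing any new hit actor implementing BPI_Enemy as TargetEnemy and moving the outline to it.
; Looking away clears the target and outline unless that enemy's BPC_Immobilise reports it immobilised, in which case it stays targeted.
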(event `self.ReceiveBeginPlay`
  (set `self.Player_Camera` (`Actor.GetComponentByClass` (`self.GetOwner`) "/Script/Engine.CameraComponent")))

(event `self.ReceiveTick`
  (params (DeltaSeconds :type "Float (single-precision)"))
  (bind _player_camera (`self.Player_Camera`))
  (bind _target_enemy (`self.Target_Enemy`))
  (bind _target_enemy_2 (`self.Target_Enemy`))
  (bind _returnvalue (`SceneComponent.K2_GetComponentLocation` _player_camera))
  (bind (_outhit _returnvalue_2) (`KismetSystemLibrary.LineTraceSingleForObjects` _returnvalue (+ _returnvalue (* (`SceneComponent.GetForwardVector` _player_camera) 5000.0)) (`|MakeArray` "ObjectTypeQuery3" "ObjectTypeQuery2" "ObjectTypeQuery1" :!type "EObjectTypeQuery Enum") false (`|MakeArray` (`self.GetOwner`)) "ForOneFrame"))
  (if _returnvalue_2
    (bind (_bblockinghit _binitialoverlap _time _distance _location _impactpoint _normal _impactnormal _physmat _hitactor) (`GameplayStatics.BreakHitResult` _outhit))
    (bind _returnvalue_3 (`KismetSystemLibrary.DoesImplementInterface` _hitactor "/Game/Characters/Enemies/Interfaces/BPI_Enemy.BPI_Enemy_C"))
    (if (and _returnvalue_3 (not _binitialoverlap) (not (== (`self.Target_Enemy`) _hitactor)))
      (`/Engine/EditorBlueprintResources/StandardMacros.IsValid` _target_enemy_2
        (:`Is Valid`
          (`MeshComponent.SetOverlayMaterial` (`Actor.GetComponentByClass` _target_enemy_2 "/Script/Engine.SkeletalMeshComponent") null))
        (:`Is Not Valid`
          _))
      (bind _output_get (set `self.Target_Enemy` _hitactor))
      (`MeshComponent.SetOverlayMaterial` (`Actor.GetComponentByClass` _output_get "/Script/Engine.SkeletalMeshComponent") "/Game/Characters/Enemies/Materials/MI_Oultine_Selected.MI_Oultine_Selected")
      (elif (not _returnvalue_3)
        (`/Engine/EditorBlueprintResources/StandardMacros.IsValid` _target_enemy
          (:`Is Valid`
            (if (not (`/Game/Characters/Enemies/Components/BPC_Immobilise.Immobilised` (`Actor.GetComponentByClass` (`self.Target_Enemy`) "/Game/Characters/Enemies/Components/BPC_Immobilise.BPC_Immobilise_C")))
              (`MeshComponent.SetOverlayMaterial` (`Actor.GetComponentByClass` _target_enemy "/Script/Engine.SkeletalMeshComponent") null)
              (set `self.Target_Enemy` null))))))
    (else
      (`/Engine/EditorBlueprintResources/StandardMacros.IsValid` (`self.Target_Enemy`)
        (:`Is Valid`
          (if (not (`/Game/Characters/Enemies/Components/BPC_Immobilise.Immobilised` (`Actor.GetComponentByClass` (`self.Target_Enemy`) "/Game/Characters/Enemies/Components/BPC_Immobilise.BPC_Immobilise_C")))
            (`MeshComponent.SetOverlayMaterial` (`Actor.GetComponentByClass` (`self.Target_Enemy`) "/Script/Engine.SkeletalMeshComponent") null)
            (set `self.Target_Enemy` null)))))))