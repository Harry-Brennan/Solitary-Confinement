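; Player component that drives two chains, left and right, to immobilise the targeted enemy.
; After a short delay on BeginPlay, it caches the owner's BPC_Enemy_Targeting component.
; Each chain input requires a valid target and toggles that side's in-use flag, calling Immobilise or StopImmobilise on the target's BPC_Immobilise.
; Chains store no enemy reference, so recall acts on whichever enemy is currently targeted.
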(event `self.ReceiveBeginPlay`
  (`KismetSystemLibrary.Delay` 0.2)
  (set `self.Enemy Targeting Component` (`Actor.GetComponentByClass` (`self.GetOwner`) "/Game/Characters/Player/Components/BPC_Enemy_Targeting.BPC_Enemy_Targeting_C")))

(event `EnhancedInput|/Game/Characters/Player/Input/Actions/IA_Left_Chain`
  (params (ActionValue :type Boolean) (ElapsedSeconds :type "Float (double-precision)") (TriggeredSeconds :type "Float (double-precision)") (InputAction :type "InputAction Object Reference" :default "/Game/Characters/Player/Input/Actions/IA_Left_Chain.IA_Left_Chain"))
  (:`Triggered`
    (`/Engine/EditorBlueprintResources/StandardMacros.IsValid` (`/Game/Characters/Player/Components/BPC_Enemy_Targeting.Target_Enemy` (`self.Enemy Targeting Component`))
      (:`Is Valid`
        (if (`self.Left_In_Use`)
          (`self.Recall_Chain` true)
          (else
            (`self.Use_Chain` true)))))))

(event `EnhancedInput|/Game/Characters/Player/Input/Actions/IA_Right_Chain`
  (params (ActionValue :type Boolean) (ElapsedSeconds :type "Float (double-precision)") (TriggeredSeconds :type "Float (double-precision)") (InputAction :type "InputAction Object Reference" :default "/Game/Characters/Player/Input/Actions/IA_Right_Chain.IA_Right_Chain"))
  (:`Triggered`
    (`/Engine/EditorBlueprintResources/StandardMacros.IsValid` (`/Game/Characters/Player/Components/BPC_Enemy_Targeting.Target_Enemy` (`self.Enemy Targeting Component`))
      (:`Is Valid`
        (if (`self.Right_In_Use`)
          (`self.Recall_Chain` false)
          (else
            (`self.Use_Chain` false)))))))

(fn `Recall_Chain`
  (params (`Left Chain` :type Boolean))
  (if `Left Chain`
    (set `self.Left_In_Use` false)
    (else
      (set `self.Right_In_Use` false)))
  (`/Game/Characters/Enemies/Components/BPC_Immobilise.Stop_Immobilise` (`Actor.GetComponentByClass` (`/Game/Characters/Player/Components/BPC_Enemy_Targeting.Target_Enemy` (`self.Enemy Targeting Component`)) "/Game/Characters/Enemies/Components/BPC_Immobilise.BPC_Immobilise_C")))

(fn `Use_Chain`
  (params (`Left Chain` :type Boolean))
  (if `Left Chain`
    (set `self.Left_In_Use` true)
    (else
      (set `self.Right_In_Use` true)))
  (`/Game/Characters/Enemies/Components/BPC_Immobilise.Immobilise` (`Actor.GetComponentByClass` (`/Game/Characters/Player/Components/BPC_Enemy_Targeting.Target_Enemy` (`self.Enemy Targeting Component`)) "/Game/Characters/Enemies/Components/BPC_Immobilise.BPC_Immobilise_C")))